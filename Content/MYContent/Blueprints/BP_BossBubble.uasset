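; BP_BossBubble is a colored bubble in the boss's shield that can detach, ease over to a minion and attach to it.
; Construction picks one of five random colors, tints the sprite and trace, and caches the BP_BOSS reference.
; A same-colored or multicolored BP_Bubble hit pops it, while overlapping the cannon deals damage and pops it.
; Destruction, immediate or randomly delayed, spawns an explosion effect and removes it from the shield array.
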(event OnComponentBeginOverlap(RootSphereColision)
  (params (OverlappedComponent :type Primitive%20Component%20Object%20Reference) (OtherActor :type Actor%20Object%20Reference) (OtherComp :type Primitive%20Component%20Object%20Reference) (OtherBodyIndex :type Integer) (bFromSweep :type Boolean) (SweepResult :type Hit%20Result%20Structure%20%28by%20ref%29))
  ;[1 1 1] CollideWithCannon
  (bind _asbp_canon (Utilities|Casting|CastToBP_Canon OtherActor))
  (Default|ChangeHealth(TakeDamage) _asbp_canon -0.01)
  (CallFunction|DestroySelf))

(event OnComponentHit(RootSphereColision)
  (params (HitComponent :type Primitive%20Component%20Object%20Reference) (OtherActor :type Actor%20Object%20Reference) (OtherComp :type Primitive%20Component%20Object%20Reference) (NormalImpulse :type Vector :default "0, 0, 0") (Hit :type Hit%20Result%20Structure%20%28by%20ref%29))
  ;[1 1 1] CollideWithShoot
  (bind _asbp_bubble (Utilities|Casting|CastToBP_Bubble OtherActor))
  (if (or (Utilities|Enum|Equal(Enum) (Variables|/Game/MYContent/Blueprints/BP_Bubble.BP_Bubble_C|GetPassedColors _asbp_bubble) (Variables|Default|GetPassedColors)) (Utilities|Enum|Equal(Enum) (Variables|/Game/MYContent/Blueprints/BP_Bubble.BP_Bubble_C|GetPassedColors _asbp_bubble) "NewEnumerator7"))
    (Game|SpawnActorfromClass "/Game/MYContent/Blueprints/Effects/BP_BubbleExplosionEffect.BP_BubbleExplosionEffect_C" (Math|Transform|MakeTransform (Transformation|GetActorLocation OtherActor) "0, 0, 0" "1,1,1") "AlwaysSpawn" 0 0)
    (Actor|DestroyActor OtherActor)
    (CallFunction|DestroySelf)))

(event Custom|MoveToBot
  (params (DestinationX :type Float%20%28single-precision%29) (DestinationZ :type Float%20%28single-precision%29) (ParentMinion :type BP%20Minion%202%20Object%20Reference))
  (bind _self self)
  (bind _rootspherecolision (Variables|Default|GetRootSphereColision))
  (bind _returnvalue (Transformation|GetWorldTransform _rootspherecolision))
  ;[1 1 1] MoveToBot
  (Transformation|DetachFromActor _self "KeepWorld" "KeepWorld" "KeepWorld")
  (Utilities|Array|AddUnique (Variables|/Game/MYContent/Blueprints/BP_Minion2.BP_Minion2_C|GetArrayOfBossBubbles ParentMinion) _self)
  (Components|MoveComponentTo (Variables|Default|GetRootSphereColision) (Math|Vector|MakeVector DestinationX (.y (.location _returnvalue)) DestinationZ) (.rotation _returnvalue) true false 3.0 false)
  (Transformation|AttachActorToActor _self ParentMinion "None" "KeepWorld" "KeepWorld" "KeepWorld" false))

(event Custom|DestroySelf
  ;[1 1 1] DestroySelf
  (Game|SpawnActorfromClass "/Game/MYContent/Blueprints/Effects/BP_BubbleExplosionEffect.BP_BubbleExplosionEffect_C" (Math|Transform|MakeTransform (Transformation|GetWorldLocation (Variables|Default|GetRootSphereColision)) "0, 0, 0" "1,1,1") "AlwaysSpawn" 0 0)
  (Utilities|Array|RemoveItem (Variables|/Game/MYContent/Blueprints/BP_BOSS.BP_BOSS_C|GetBossShieldBubble (Variables|Default|GetRefToBoss)) self)
  (Actor|DestroyActor))

(event Custom|DelayedSelfDestruction
  ;[1 1 1] DelayedSelfDestruction
  (Utilities|FlowControl|Delay (Math|Random|RandomFloatinRange 0.0 1.5))
  (Game|SpawnActorfromClass "/Game/MYContent/Blueprints/Effects/BP_BubbleExplosionEffect.BP_BubbleExplosionEffect_C" (Math|Transform|MakeTransform (Transformation|GetWorldLocation (Variables|Default|GetRootSphereColision)) "0, 0, 0" "1,1,1") "AlwaysSpawn" 0 0)
  (Utilities|Array|RemoveItem (Variables|/Game/MYContent/Blueprints/BP_BOSS.BP_BOSS_C|GetBossShieldBubble (Variables|Default|GetRefToBoss)) self)
  (Actor|DestroyActor))

(fn ConstructionScript
  (bind _papersprite (Variables|Default|GetPaperSprite))
  (switch int (Math|Random|RandomInteger 5)
    (:0
      (Variables|Default|SetPassedColors "NewEnumerator0"))
    (:1
      (Variables|Default|SetPassedColors "NewEnumerator1"))
    (:2
      (Variables|Default|SetPassedColors "NewEnumerator2"))
    (:3
      (Variables|Default|SetPassedColors "NewEnumerator3"))
    (:4
      (Variables|Default|SetPassedColors "NewEnumerator4")))
  (switch Utilities|FlowControl|Switch|SwitchonEnumColors (Variables|Default|GetPassedColors)
    (:NewEnumerator0
      (Sprite|SetSpriteColor _papersprite (Utilities|Struct|MakeLinearColor 1.0 0.0 0.0 1.0)))
    (:NewEnumerator1
      (Sprite|SetSpriteColor _papersprite (Utilities|Struct|MakeLinearColor 0.0 0.5 1.0 1.0)))
    (:NewEnumerator2
      (Sprite|SetSpriteColor _papersprite (Utilities|Struct|MakeLinearColor 0.1 1.0 0.0 1.0)))
    (:NewEnumerator3
      (Sprite|SetSpriteColor _papersprite (Utilities|Struct|MakeLinearColor 0.97 1.0 0.0 1.0)))
    (:NewEnumerator4
      (Sprite|SetSpriteColor _papersprite (Utilities|Struct|MakeLinearColor 0.98 0.33 0.0 1.0))))
  (Effects|Components|ParticleSystem|SetColorParameter (Variables|Default|GetTrace) "PassColor" (Variables|/Script/Paper2D.PaperSpriteComponent|GetSpriteColor (Variables|Default|GetPaperSprite)))
  (bind _outactors (Actor|GetAllActorsOfClass "/Game/MYContent/Blueprints/BP_BOSS.BP_BOSS_C"))
  (Variables|Default|SetRefToBoss (Utilities|Array|Get(acopy) _outactors))
  (Components|Timeline|SetLooping (Variables|Default|GetPaperFlipbook) false))