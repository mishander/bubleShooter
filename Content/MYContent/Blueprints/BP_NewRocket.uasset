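; BP_NewRocket is a rocket actor that explodes and destroys itself on contact with a BP_Canon.
; Its Top and Bottom components act as query-only overlap triggers, while the construction script disables collision on the flipbook and cube.
; Either trigger spawns BP_Explosion, with X and Z midway between the sweep location and cannon cube plus random jitter, and Y slightly offset from the sweep location.
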(event OnComponentBeginOverlap(Top)
  (params (OverlappedComponent :type Primitive%20Component%20Object%20Reference) (OtherActor :type Actor%20Object%20Reference) (OtherComp :type Primitive%20Component%20Object%20Reference) (OtherBodyIndex :type Integer) (bFromSweep :type Boolean) (SweepResult :type Hit%20Result%20Structure%20%28by%20ref%29))
  (bind (_x _y _z) (Math|Vector|BreakVector (.location SweepResult)))
  ;[1 1 1] RocketHitCannon
  (bind _asbp_canon (Utilities|Casting|CastToBP_Canon OtherActor))
  (Game|SpawnActorfromClass "/Game/MYContent/Blueprints/Effects/BP_Explosion.BP_Explosion_C" (Math|Transform|MakeTransform (Math|Vector|MakeVector (|(((A+B)/2)+C) _x (.x (Transformation|GetWorldLocation (Variables|/Game/MYContent/Blueprints/BP_Canon.BP_Canon_C|GetCube _asbp_canon))) (Math|Random|RandomFloatinRange -5.0 5.0)) (+ _y 5.0) (|(((A+B)/2)+C) _z (.z (Transformation|GetWorldLocation (Variables|/Game/MYContent/Blueprints/BP_Canon.BP_Canon_C|GetCube _asbp_canon))) (Math|Random|RandomFloatinRange -5.0 5.0))) "0, 0, 0" "1,1,1") "AlwaysSpawn" 0 0)
  (Actor|DestroyActor))

(event OnComponentBeginOverlap(Bottom)
  (params (OverlappedComponent :type Primitive%20Component%20Object%20Reference) (OtherActor :type Actor%20Object%20Reference) (OtherComp :type Primitive%20Component%20Object%20Reference) (OtherBodyIndex :type Integer) (bFromSweep :type Boolean) (SweepResult :type Hit%20Result%20Structure%20%28by%20ref%29))
  (bind (_x _y _z) (Math|Vector|BreakVector (.location SweepResult)))
  ;[1 1 1] RocketHitCannon
  (bind _asbp_canon (Utilities|Casting|CastToBP_Canon OtherActor))
  (Game|SpawnActorfromClass "/Game/MYContent/Blueprints/Effects/BP_Explosion.BP_Explosion_C" (Math|Transform|MakeTransform (Math|Vector|MakeVector (|(((A+B)/2)+C) _x (.x (Transformation|GetWorldLocation (Variables|/Game/MYContent/Blueprints/BP_Canon.BP_Canon_C|GetCube _asbp_canon))) (Math|Random|RandomFloatinRange -5.0 5.0)) (+ _y 5.0) (|(((A+B)/2)+C) _z (.z (Transformation|GetWorldLocation (Variables|/Game/MYContent/Blueprints/BP_Canon.BP_Canon_C|GetCube _asbp_canon))) (Math|Random|RandomFloatinRange -5.0 5.0))) "0, 0, 0" "1,1,1") "AlwaysSpawn" 0 0)
  (Actor|DestroyActor))

(fn ConstructionScript
  (Collision|SetCollisionEnabled (Variables|Default|GetTop) "QueryOnly")
  (Collision|SetCollisionEnabled (Variables|Default|GetBottom) "QueryOnly")
  (Collision|SetCollisionEnabled (Variables|Default|GetPaperFlipbook) "NoCollision")
  (Collision|SetCollisionEnabled (Variables|Default|GetCube) "NoCollision"))