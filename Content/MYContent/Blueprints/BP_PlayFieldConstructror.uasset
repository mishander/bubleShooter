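; Playfield manager for a bubble shooter that builds the bubble grid, spawns and launches shots, and tracks score.
; Staggered rows of random-colour bubbles link to neighbours by distance and attach to an invisible root actor.
; A recursive flood fill from the newest row finds unlinked bubbles to drop; flagged colour matches drop with score text.
; While the lowest bubble is too high, it adds rows and shifts the root down.
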(event Custom|CreateLine
  (bind _levelstartposition (Variables|Default|GetLevelStartPosition))
  ;[1 1 1] Respawn1Line
  (for _index (range 1 (Variables|Default|GetBubblesInLine))
    (if (< (Math|Random|RandomInteger 6) 5)
      (bind _returnvalue (Game|SpawnActorfromClass "/Game/MYContent/Blueprints/BP_Bubble.BP_Bubble_C" (Math|Transform|MakeTransform (Math|Vector|MakeVector (+ (+ (* (Math|Integer|%(Integer) (Variables|Default|GetDisplacement) 2) 22.0) (.x _levelstartposition)) (* _index 44.0)) 0.0 (+ (.z _levelstartposition) (* (Variables|Default|GetNumberOfRowsRespawned) 38.0))) "0, 0, 0" "1,1,1") "AlwaysSpawn" 0 0))
      ;[1 1 1] DrawingBalls
      (CallFunction|GetRandomColor)
      (Default|ChangebubbleColor _returnvalue)
      ;[1 1 1] MassiveOfBubbles
      (Components|Movement|StopMovementImmediately (Variables|/Game/MYContent/Blueprints/BP_Bubble.BP_Bubble_C|GetProjectileMovement _returnvalue))
      (if (Utilities|Enum|NotEqual(Enum) (Variables|/Game/MYContent/Blueprints/BP_Bubble.BP_Bubble_C|GetPassedColors _returnvalue) "NewEnumerator5")
        (Variables|/Game/MYContent/Blueprints/BP_Bubble.BP_Bubble_C|SetRootingBubble _returnvalue true)
        (CallFunction|AddtoPlayFieldArray _returnvalue)
        (Transformation|AttachActorToActor _returnvalue (Variables|Default|GetRefToInvisibleSceneRoot) "None" "KeepWorld" "KeepWorld" "KeepWorld" false))))
  (bind _result (Math|Integer|IncrementInt (Variables|Default|GetNumberOfRowsRespawned))
    (:%20%20
      (Variables|Default|SetNumberOfRowsRespawned _result)
      (bind _result_2 (Math|Integer|IncrementInt (Variables|Default|GetDisplacement))
        (:%20%20
          (Variables|Default|SetDisplacement _result_2))))))

(event Custom|CheckIfWeNeedToRespawnLine
  ;[1 1 1] CheckIfWeNeedToRespawnLine
  (Utilities|Array|Clear (Variables|Default|GetArrayForCountMinZ))
  (bind _array_element (Utilities|Array|ForEachLoopwithBreak (Variables|Default|GetBubblesOnPlayField))
    (:LoopBody
      (Utilities|Array|Add (Variables|Default|GetArrayForCountMinZ) (.z (Transformation|GetWorldLocation (Variables|/Game/MYContent/Blueprints/BP_Bubble.BP_Bubble_C|GetPaperSprite _array_element)))))
    (:Completed
      (if (<= (.MinValue (Math|Float|MinOfFloatArray (Variables|Default|GetArrayForCountMinZ))) (+ (.z (Variables|Default|GetLevelStartPosition)) 25.0))
        (bind _outactors (Actor|GetAllActorsOfClass "/Game/MYContent/Blueprints/BP_Canon.BP_Canon_C"))
        (Variables|/Game/MYContent/Blueprints/BP_Canon.BP_Canon_C|SetCannonState (Utilities|Array|Get(acopy) _outactors) "NewEnumerator1")
        (else
          (CallFunction|CreateNewLineOfRootingBubbles)
          (Variables|Default|SetNumberOfRowsRespawned (- (Variables|Default|GetNumberOfRowsRespawned) 1))
          (Transformation|AddActorWorldOffset (Variables|Default|GetRefToInvisibleSceneRoot) (Math|Vector|MakeVector 0.0 0.0 -38.0))
          (CallFunction|CheckifWeNeedtoRespawnLine))))))

(event Custom|KillBubble
  (params (RefToBubble :type BP%20Bubble%20Object%20Reference))
  ;[1 1 1] KillBubble
  (Utilities|Array|RemoveItem (Variables|Default|GetBubblesOnPlayField) RefToBubble)
  (for _array_element (Variables|Default|GetBubblesOnPlayField)
    (Utilities|Array|RemoveItem (Variables|/Game/MYContent/Blueprints/BP_Bubble.BP_Bubble_C|GetBubbleNeighbours _array_element) RefToBubble)
    (Collision|SetCollisionEnabled (Variables|/Game/MYContent/Blueprints/BP_Bubble.BP_Bubble_C|GetPaperSprite RefToBubble) "QueryOnly")
    (Physics|SetSimulatePhysics (Variables|/Game/MYContent/Blueprints/BP_Bubble.BP_Bubble_C|GetPaperSprite RefToBubble) true)
    (Physics|SetEnableGravity (Variables|/Game/MYContent/Blueprints/BP_Bubble.BP_Bubble_C|GetPaperSprite RefToBubble) true)))

(event Custom|CreateNewLineOfRootingBubbles
  ;[1 1 1] CreateNewLineOfRootingBubbles
  (for _array_element (Variables|Default|GetBubblesOnPlayField)
    (Variables|/Game/MYContent/Blueprints/BP_Bubble.BP_Bubble_C|SetRootingBubble _array_element false))
  (CallFunction|CreateLine))

(event Custom|KillUnlinkedBubbles
  ;[1 1 1] KillUnlinkedBubbles
  (bind _outactors (Actor|GetAllActorsOfClass "/Game/MYContent/Blueprints/BP_Bubble.BP_Bubble_C"))
  (for _array_element _outactors
    (if (Math|Boolean|NotEqual(Boolean) (Variables|/Game/MYContent/Blueprints/BP_Bubble.BP_Bubble_C|GetLinkedToRoot _array_element) true)
      (CallFunction|KillBubble _array_element))))

(event Custom|SpawnRandomBubbleForShooting
  (bind _returnvalue (Game|GetPlayerController 0))
  (bind _returnvalue_2 (Transformation|GetActorTransform _returnvalue))
  ;[1 1 1] SpawnShootBubble
  (Actor|GetAllActorsOfClass "/Game/MYContent/Blueprints/BP_Canon.BP_Canon_C")
  (bind _returnvalue_3 (Game|SpawnActorfromClass "/Game/MYContent/Blueprints/BP_Bubble.BP_Bubble_C" (Math|Transform|MakeTransform (Math|Vector|MakeVector (.x (.location _returnvalue_2)) (+ (.y (.location _returnvalue_2)) 1.0) (.z (.location _returnvalue_2))) "0, 0, 0" "1.000000,1,1") "Undefined" 0 0))
  ;[1 1 1] SetCollorToShootingBubble
  (switch int (Math|Random|RandomInteger 5)
    (:0
      (Variables|/Game/MYContent/Blueprints/BP_Bubble.BP_Bubble_C|SetPassedColors _returnvalue_3 "NewEnumerator0"))
    (:1
      (Variables|/Game/MYContent/Blueprints/BP_Bubble.BP_Bubble_C|SetPassedColors _returnvalue_3 "NewEnumerator1"))
    (:2
      (Variables|/Game/MYContent/Blueprints/BP_Bubble.BP_Bubble_C|SetPassedColors _returnvalue_3 "NewEnumerator2"))
    (:3
      (Variables|/Game/MYContent/Blueprints/BP_Bubble.BP_Bubble_C|SetPassedColors _returnvalue_3 "NewEnumerator3"))
    (:4
      (Variables|/Game/MYContent/Blueprints/BP_Bubble.BP_Bubble_C|SetPassedColors _returnvalue_3 "NewEnumerator4")))
  (Default|ChangebubbleColor _returnvalue_3)
  (Collision|SetCollisionEnabled (Variables|/Game/MYContent/Blueprints/BP_Bubble.BP_Bubble_C|GetPaperSprite _returnvalue_3) "NoCollision")
  (Variables|/Game/MYContent/Blueprints/BP_Bubble.BP_Bubble_C|SetRootingBubble _returnvalue_3 false)
  (Variables|/Game/MYContent/Blueprints/BP_Bubble.BP_Bubble_C|SetLinkedToRoot _returnvalue_3 true)
  (Default|StopProjectile _returnvalue_3))

(event Custom|PlaceCorners
  (bind _returnvalue (Game|GetPlayerController 0))
  (bind _returnvalue_2 (Game|GetPlayerController 0))
  (bind _returnvalue_3 (Transformation|GetActorTransform _returnvalue))
  (bind _returnvalue_4 (Transformation|GetActorTransform _returnvalue_2))
  ;[1 1 1] PlaceCorners
  (bind _returnvalue_5 (Game|SpawnActorfromClass "/Game/MYContent/Blueprints/BlackCorners.BlackCorners_C" (Math|Transform|MakeTransform (Math|Vector|MakeVector (+ (.x (.location _returnvalue_4)) -4e+02) (.y (.location _returnvalue_4)) (.z (.location _returnvalue_4))) "0, 0, 0" "1,1,20.000000") "AlwaysSpawn" 0 0))
  (Sprite|SetSpriteColor (Variables|/Game/MYContent/Blueprints/BlackCorners.BlackCorners_C|GetPaperSprite _returnvalue_5) (Utilities|Struct|MakeLinearColor (.r (Variables|/Script/Paper2D.PaperSpriteComponent|GetSpriteColor (Variables|/Game/MYContent/Blueprints/BlackCorners.BlackCorners_C|GetPaperSprite _returnvalue_5))) (.g (Variables|/Script/Paper2D.PaperSpriteComponent|GetSpriteColor (Variables|/Game/MYContent/Blueprints/BlackCorners.BlackCorners_C|GetPaperSprite _returnvalue_5))) (.b (Variables|/Script/Paper2D.PaperSpriteComponent|GetSpriteColor (Variables|/Game/MYContent/Blueprints/BlackCorners.BlackCorners_C|GetPaperSprite _returnvalue_5))) 0.5))
  (bind _returnvalue_6 (Game|SpawnActorfromClass "/Game/MYContent/Blueprints/BlackCorners.BlackCorners_C" (Math|Transform|MakeTransform (Math|Vector|MakeVector (+ (.x (.location _returnvalue_3)) 4e+02) (.y (.location _returnvalue_3)) (.z (.location _returnvalue_3))) "0, 0, 0" "1,1,20.000000") "AlwaysSpawn" 0 0))
  (Sprite|SetSpriteColor (Variables|/Game/MYContent/Blueprints/BlackCorners.BlackCorners_C|GetPaperSprite _returnvalue_6) (Utilities|Struct|MakeLinearColor (.r (Variables|/Script/Paper2D.PaperSpriteComponent|GetSpriteColor (Variables|/Game/MYContent/Blueprints/BlackCorners.BlackCorners_C|GetPaperSprite _returnvalue_6))) (.g (Variables|/Script/Paper2D.PaperSpriteComponent|GetSpriteColor (Variables|/Game/MYContent/Blueprints/BlackCorners.BlackCorners_C|GetPaperSprite _returnvalue_6))) (.b (Variables|/Script/Paper2D.PaperSpriteComponent|GetSpriteColor (Variables|/Game/MYContent/Blueprints/BlackCorners.BlackCorners_C|GetPaperSprite _returnvalue_6))) 0.5)))

(event Custom|GetRandomColor
  ;[1 1 1] DrawingBalls
  (switch int (Math|Random|RandomInteger 5)
    (:0
      (Variables|/Game/MYContent/Blueprints/BP_Bubble.BP_Bubble_C|SetPassedColors (stale Custom|CreateLine _returnvalue) "NewEnumerator0"))
    (:1
      (Variables|/Game/MYContent/Blueprints/BP_Bubble.BP_Bubble_C|SetPassedColors (stale Custom|CreateLine _returnvalue) "NewEnumerator1"))
    (:2
      (Variables|/Game/MYContent/Blueprints/BP_Bubble.BP_Bubble_C|SetPassedColors (stale Custom|CreateLine _returnvalue) "NewEnumerator2"))
    (:3
      (Variables|/Game/MYContent/Blueprints/BP_Bubble.BP_Bubble_C|SetPassedColors (stale Custom|CreateLine _returnvalue) "NewEnumerator3"))
    (:4
      (Variables|/Game/MYContent/Blueprints/BP_Bubble.BP_Bubble_C|SetPassedColors (stale Custom|CreateLine _returnvalue) "NewEnumerator4"))))

(event Custom|BuildLinksFromRoot
  ;[1 1 1] CheckRooted
  ;;[1 1 1] BuildLinksFromRoot
  (for _array_element (Variables|Default|GetBubblesOnPlayField)
    (if (Variables|/Game/MYContent/Blueprints/BP_Bubble.BP_Bubble_C|GetLinkedToRoot _array_element)
      (for _array_element_2 (Variables|/Game/MYContent/Blueprints/BP_Bubble.BP_Bubble_C|GetBubbleNeighbours _array_element)
        (if (not (Variables|/Game/MYContent/Blueprints/BP_Bubble.BP_Bubble_C|GetLinkedToRoot _array_element_2))
          (Variables|/Game/MYContent/Blueprints/BP_Bubble.BP_Bubble_C|SetLinkedToRoot _array_element_2 true)
          (CallFunction|BuildLinksfromRoot))))))

(event Custom|UnlinkAll
  ;[1 1 1] UnlinkAllTMP
  (for _array_element (Variables|Default|GetBubblesOnPlayField)
    (Variables|/Game/MYContent/Blueprints/BP_Bubble.BP_Bubble_C|SetLinkedToRoot _array_element false)))

(event Custom|AddToPlayFieldArray
  (params (BubbleRef :type BP%20Bubble%20Object%20Reference))
  ;[1 1 1] MassiveOfBubbles
  (Utilities|Array|AddUnique (Variables|Default|GetBubblesOnPlayField) BubbleRef)
  (for _array_element (Variables|Default|GetBubblesOnPlayField)
    (if (Math|Boolean|ANDBoolean (!= (Transformation|GetDistanceTo BubbleRef _array_element) 0.0) (< (Transformation|GetDistanceTo BubbleRef _array_element) 5e+01) (Utilities|Enum|NotEqual(Enum) (Variables|/Game/MYContent/Blueprints/BP_Bubble.BP_Bubble_C|GetPassedColors BubbleRef) "NewEnumerator5") (Utilities|Enum|NotEqual(Enum) (Variables|/Game/MYContent/Blueprints/BP_Bubble.BP_Bubble_C|GetPassedColors _array_element) "NewEnumerator5"))
      (Utilities|Array|AddUnique (Variables|/Game/MYContent/Blueprints/BP_Bubble.BP_Bubble_C|GetBubbleNeighbours BubbleRef) _array_element)
      (Utilities|Array|AddUnique (Variables|/Game/MYContent/Blueprints/BP_Bubble.BP_Bubble_C|GetBubbleNeighbours _array_element) BubbleRef))))

(event Custom|AddPoints
  (params (AddedScores :type Integer))
  ;[1 1 1] AddPoints
  (Variables|Default|SetPlayerScores (+ (Variables|Default|GetPlayerScores) AddedScores)))

(event Custom|CheckRooted
  ;[1 1 1] CheckRooted
  (CallFunction|UnlinkAll)
  (for _array_element (Variables|Default|GetBubblesOnPlayField)
    (if (and (Variables|/Game/MYContent/Blueprints/BP_Bubble.BP_Bubble_C|GetRootingBubble _array_element) (Math|Boolean|NotEqual(Boolean) (Variables|/Game/MYContent/Blueprints/BP_Bubble.BP_Bubble_C|GetLinkedToRoot _array_element) true))
      (Variables|/Game/MYContent/Blueprints/BP_Bubble.BP_Bubble_C|SetLinkedToRoot _array_element true)))
  (CallFunction|BuildLinksfromRoot))

(event Custom|KillBubblesOfTheSameColor
  ;[1 1 1] KillBubblesOfTheSameColor
  (bind _outactors (Actor|GetAllActorsOfClass "/Game/MYContent/Blueprints/BP_Bubble.BP_Bubble_C"))
  (for _array_element _outactors
    (if (Variables|/Game/MYContent/Blueprints/BP_Bubble.BP_Bubble_C|GetProjectileNeedToBeRemoved _array_element)
      (bind _returnvalue (Game|SpawnActorfromClass "/Game/MYContent/Blueprints/BP_textObject.BP_textObject_C" (Math|Transform|MakeTransform (.location (Transformation|GetWorldTransform (Variables|/Game/MYContent/Blueprints/BP_Bubble.BP_Bubble_C|GetPaperSprite _array_element))) (Math|Rotator|MakeRotator (.roll (.rotation (Transformation|GetWorldTransform (Variables|/Game/MYContent/Blueprints/BP_Bubble.BP_Bubble_C|GetPaperSprite _array_element)))) 0.0 (+ (.yaw (.rotation (Transformation|GetWorldTransform (Variables|/Game/MYContent/Blueprints/BP_Bubble.BP_Bubble_C|GetPaperSprite _array_element)))) 9e+01)) "1,1,1") "AlwaysSpawn" 0 0))
      (Rendering|Components|TextRender|SetTextRenderColor (Variables|/Game/MYContent/Blueprints/BP_textObject.BP_textObject_C|GetTextRender _returnvalue) (Math|Conversions|ToColor(LinearColor) (Variables|/Script/Paper2D.PaperSpriteComponent|GetSpriteColor (Variables|/Game/MYContent/Blueprints/BP_Bubble.BP_Bubble_C|GetPaperSprite _array_element))))
      (Rendering|Components|TextRender|SetText (Variables|/Game/MYContent/Blueprints/BP_textObject.BP_textObject_C|GetTextRender _returnvalue) (Variables|Default|GetScoresFromDestroyingBubble))
      (Variables|/Game/MYContent/Blueprints/BP_Bubble.BP_Bubble_C|SetPassedColors _array_element "NewEnumerator6")
      (Default|ChangebubbleColor _array_element)
      (CallFunction|KillBubble _array_element))))

(event Custom|LaunchBubble
  ;[1 1 1] LaunchBubble
  (bind _outactors (Actor|GetAllActorsOfClass "/Game/MYContent/Blueprints/BP_Canon.BP_Canon_C"))
  (Transformation|SetActorTransform (stale Custom|SpawnRandomBubbleForShooting _returnvalue_3) (Math|Transform|MakeTransform (Math|Vector|MakeVector (.x (.location (Transformation|GetWorldTransform (Variables|/Game/MYContent/Blueprints/BP_Canon.BP_Canon_C|GetCube (Utilities|Array|Get(acopy) _outactors))))) (+ (.y (.location (Transformation|GetWorldTransform (Variables|/Game/MYContent/Blueprints/BP_Canon.BP_Canon_C|GetCube (Utilities|Array|Get(acopy) _outactors))))) 1.0) (.z (.location (Transformation|GetWorldTransform (Variables|/Game/MYContent/Blueprints/BP_Canon.BP_Canon_C|GetCube (Utilities|Array|Get(acopy) _outactors)))))) (.rotation (Transformation|GetWorldTransform (Variables|/Game/MYContent/Blueprints/BP_Canon.BP_Canon_C|GetCube (Utilities|Array|Get(acopy) _outactors)))) (.scale (Transformation|GetWorldTransform (Variables|/Game/MYContent/Blueprints/BP_Canon.BP_Canon_C|GetCube (Utilities|Array|Get(acopy) _outactors))))))
  (Collision|SetCollisionEnabled (Variables|/Game/MYContent/Blueprints/BP_Bubble.BP_Bubble_C|GetPaperSprite (stale Custom|SpawnRandomBubbleForShooting _returnvalue_3)) "QueryOnly")
  (Variables|/Script/Engine.ProjectileMovementComponent|SetbShouldBounce (Variables|/Game/MYContent/Blueprints/BP_Bubble.BP_Bubble_C|GetProjectileMovement (stale Custom|SpawnRandomBubbleForShooting _returnvalue_3)) true)
  (Variables|/Script/Engine.ProjectileMovementComponent|SetMaxSpeed (Variables|/Game/MYContent/Blueprints/BP_Bubble.BP_Bubble_C|GetProjectileMovement (stale Custom|SpawnRandomBubbleForShooting _returnvalue_3)) 1.2e+03)
  (Game|Components|ProjectileMovement|SetVelocityinLocalSpace (Variables|/Game/MYContent/Blueprints/BP_Bubble.BP_Bubble_C|GetProjectileMovement (stale Custom|SpawnRandomBubbleForShooting _returnvalue_3)) "0.0,0.0,750.0"))

(event EventBeginPlay
  ;[1 1 1] Start Game Event
  (Variables|/Script/Engine.PlayerController|SetbShowMouseCursor (Game|GetPlayerController 0) true)
  (for _index (range 1 (Variables|Default|GetNumberOfColumns))
    (CallFunction|CreateNewLineOfRootingBubbles))
  (CallFunction|CheckRooted)
  (CallFunction|KillUnlinkedBubbles)
  (bind _returnvalue (UserInterface|CreateWidget "/Game/MYContent/Blueprints/InterfaceWidget.InterfaceWidget_C" (Game|GetPlayerController 0)))
  (UserInterface|Viewport|AddtoViewport _returnvalue 0)
  (CallFunction|PlaceCorners))

(fn ConstructionScript
  (bind _outactors (Actor|GetAllActorsOfClass "/Game/MYContent/Blueprints/InvisibleSceneRoot.InvisibleSceneRoot_C"))
  (Variables|Default|SetRefToInvisibleSceneRoot (Utilities|Array|Get(acopy) _outactors))
  (Transformation|SetActorLocation (Variables|Default|GetRefToInvisibleSceneRoot) (Variables|Default|GetLevelStartPosition) false false))