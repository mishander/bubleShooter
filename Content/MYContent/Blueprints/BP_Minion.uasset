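; BP_Minion is an enemy ship that flies into position, faces BP_Canon and repeatedly fires rockets.
; MoveActorToLocation eases the Sphere to a destination, then enables its collision and starts BattleScript.
; BattleScript loops through chained timelines: random vertical drift biased toward StartingZ, stop, pause, request a rocket from BP_RocketManager, pause.
; Tick keeps it aimed at the cannon and repositions engine particles by the sign of X.
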(event Custom|MoveActorToLocation
  (params (DestinationX :type Float%20%28single-precision%29) (DestinationZ :type Float%20%28single-precision%29) (Time :type Float%20%28single-precision%29))
  (bind _sphere (Variables|Default|GetSphere))
  (bind _sphere_2 (Variables|Default|GetSphere))
  (bind _returnvalue (Transformation|GetWorldLocation _sphere))
  (bind _returnvalue_2 (Math|Rotator|FindLookatRotation (Math|Vector|MakeVector (.x _returnvalue) (.y _returnvalue) (.z _returnvalue)) (Math|Vector|MakeVector DestinationX -3.0 DestinationZ)))
  (bind (_roll _pitch _yaw) (Math|Rotator|BreakRotator _returnvalue_2))
  ;[1 1 1] MoveToLocation
  (Transformation|SetWorldRotation _sphere_2 (Math|Rotator|MakeRotator _roll (+ _pitch 2.7e+02) _yaw) false false)
  (Components|MoveComponentTo (Variables|Default|GetSphere) (Math|Vector|MakeVector DestinationX 0.0 DestinationZ) (Transformation|GetWorldRotation _sphere_2) true false Time false)
  (CallFunction|RotatetoCannon))

(event Custom|BattleScript
  ;[1 1 1] BattleScript
  (CallFunction|DeltaZforMovement)
  (Timeline|TimeForMovement PlayFromStart
    (:Finished
      (Components|Movement|StopMovementImmediately (Variables|Default|GetProjectileMovement))
      (Timeline|TimeBeforeShot PlayFromStart
        (:Finished
          (CallFunction|Shot)
          (Timeline|TimeAfterShot PlayFromStart
            (:Finished
              (CallFunction|BattleScript))))))))

(event Custom|RotateToCannon
  (bind _returnvalue (Transformation|GetActorLocation))
  (bind _reftocannon (Variables|Default|GetRefToCannon))
  (bind _returnvalue_2 (Transformation|GetActorLocation _reftocannon))
  (bind _returnvalue_3 (Math|Rotator|FindLookatRotation (Math|Vector|MakeVector (.x _returnvalue) (.y _returnvalue) (.z _returnvalue)) _returnvalue_2))
  (bind (_roll _pitch _yaw) (Math|Rotator|BreakRotator _returnvalue_3))
  ;[1 1 1] RotateToCannon
  ;;[1 1 1] NeedToUseInterpolateHere
  (Transformation|SetWorldRotation (Variables|Default|GetSphere) (Math|Rotator|MakeRotator _roll (+ _pitch 2.7e+02) _yaw) false false)
  (Variables|Default|SetOnPosition true)
  (Collision|SetCollisionEnabled (Variables|Default|GetSphere) "QueryAndPhysics")
  (CallFunction|BattleScript))

(event Custom|Shot
  ;[1 1 1] Shot
  (Default|RespawnRocket (Variables|Default|GetRefToRocketManager) (Transformation|GetActorLocation self)))

(event Custom|DeltaZForMovement
  (bind _self self)
  (bind _startingz (Variables|Default|GetStartingZ))
  (bind _returnvalue (Transformation|GetActorLocation _self))
  (bind _returnvalue_2 (- (.z _returnvalue) _startingz))
  ;[1 1 1] DeltaZForMovement
  (Variables|/Script/Engine.MovementComponent|SetVelocity (Variables|Default|GetProjectileMovement) (Math|Vector|MakeVector 0.0 0.0 (Math|Random|RandomFloatinRange (- -1e+02 _returnvalue_2) (- 3e+02 _returnvalue_2)))))

(event EventTick
  (params (DeltaSeconds :type Float%20%28single-precision%29))
  (bind _returnvalue (Transformation|GetActorLocation))
  (bind _reftocannon (Variables|Default|GetRefToCannon))
  (bind _returnvalue_2 (Transformation|GetActorLocation _reftocannon))
  (bind _returnvalue_3 (Math|Rotator|FindLookatRotation (Math|Vector|MakeVector (.x _returnvalue) (.y _returnvalue) (.z _returnvalue)) _returnvalue_2))
  (bind (_roll _pitch _yaw) (Math|Rotator|BreakRotator _returnvalue_3))
  ;[1 1 1] FixIssueWithEngineParticles
  (Utilities|FlowControl|Sequence
    (:then_0
      (if (>= (.x (Transformation|GetActorLocation)) 0.0)
        (Transformation|SetRelativeLocation (Variables|Default|GetP_Right) (Math|Vector|MakeVector 17.0 2.0 -66.0) false false)
        (Transformation|SetRelativeLocation (Variables|Default|GetP_Left) (Math|Vector|MakeVector -16.0 2.0 -66.0) false false)
        (else
          (Transformation|SetRelativeLocation (Variables|Default|GetP_Right) (Math|Vector|MakeVector 17.0 -2.0 -66.0) false false)
          (Transformation|SetRelativeLocation (Variables|Default|GetP_Left) (Math|Vector|MakeVector -16.0 -2.0 -66.0) false false))))
    (:then_1
      (if (Variables|Default|GetOnPosition)
        (Transformation|SetWorldRotation (Variables|Default|GetSphere) (Math|Rotator|MakeRotator _roll (+ _pitch 2.7e+02) _yaw) false false)))))

(fn ConstructionScript
  (Effects|Components|ParticleSystem|SetColorParameter (Variables|Default|GetP_Right) "PassColor" (Utilities|Struct|MakeLinearColor 0.0 0.5 1.0 1.0))
  (Effects|Components|ParticleSystem|SetColorParameter (Variables|Default|GetP_Left) "PassColor" (Utilities|Struct|MakeLinearColor 0.0 0.5 1.0 1.0))
  (bind _outactors (Actor|GetAllActorsOfClass "/Game/MYContent/Blueprints/BP_Canon.BP_Canon_C"))
  (Variables|Default|SetRefToCannon (Utilities|Array|Get(acopy) _outactors))
  (bind _outactors_2 (Actor|GetAllActorsOfClass "/Game/MYContent/Blueprints/BP_RocketManager.BP_RocketManager_C"))
  (Variables|Default|SetRefToRocketManager (Utilities|Array|Get(acopy) _outactors_2)))