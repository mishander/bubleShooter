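; BP_SunMarker is a temporary moving marker that turns into a BP_Sun at its destination.
; MoveActorToLocationPerTime moves the Sphere component, not the actor root, to a relative X/Z on a fixed Y plane over a given time, then calls SpwanSun.
; SpwanSun spawns BP_Sun at the Sphere's world location and destroys the marker.
; The construction script shrinks the Sphere and tints PRight and PLeft blue.
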(event Custom|MoveActorToLocationPerTime
  (params (DestinationX :type Float%20%28single-precision%29) (DestinationZ :type Float%20%28single-precision%29) (Time :type Float%20%28single-precision%29))
  ;[1 1 1] MoveTO
  (Components|MoveComponentTo (Variables|Default|GetSphere) (Math|Vector|MakeVector DestinationX -2.0 DestinationZ) "0.000000, 0,180.000000" false false Time false)
  (CallFunction|SpwanSun))

(event Custom|SpwanSun
  ;[1 1 1] SpwanSun
  (Game|SpawnActorfromClass "/Game/MYContent/Blueprints/BP_Sun.BP_Sun_C" (Math|Transform|MakeTransform (Transformation|GetWorldLocation (Variables|Default|GetSphere)) "0, 0, 0" "1,1,1") "AlwaysSpawn" 0 0)
  (Actor|DestroyActor))

(fn ConstructionScript
  (Effects|Components|ParticleSystem|SetColorParameter (Variables|Default|GetP_Right) "PassColor" (Utilities|Struct|MakeLinearColor 0.0 0.5 1.0 1.0))
  (Effects|Components|ParticleSystem|SetColorParameter (Variables|Default|GetP_Left) "PassColor" (Utilities|Struct|MakeLinearColor 0.0 0.5 1.0 1.0))
  (Transformation|SetWorldScale3D (Variables|Default|GetSphere) "0.250000,0.250000,0.250000"))