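; BP_SpecialBubbleTextObject is a short-lived pop-up text actor that grows and flashes random colours.
; A looping timer from BeginPlay interpolates the TextRender world size upward and randomises its colour until a size threshold is reached.
; It then clears the timer, slides the text to a fixed relative location, hides it, sets IsButtonActive on the BP_PlayFieldConstructror found at construction, and destroys itself.
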(event Custom|MakeTextBigger
  (bind _textrender (Variables|Default|GetTextRender))
  (bind _deltat (Variables|Default|GetDeltaT))
  (bind _textrender_2 (Variables|Default|GetTextRender))
  (bind _worldsize (Variables|/Script/Engine.TextRenderComponent|GetWorldSize _textrender))
  (bind _returnvalue (Math|Interpolation|FInterptoConstant _worldsize 4.5e+02 _deltat 1.5e+02))
  ;[1 1 1] ChangeBubbleColorAndSize
  (if (< _returnvalue 3.5e+02)
    (Rendering|Components|TextRender|SetWorldSize _textrender _returnvalue)
    (Rendering|Components|TextRender|SetTextRenderColor (Variables|Default|GetTextRender) (Math|Color|MakeColor (Math|Conversions|ToByte(Integer) (Math|Random|RandomIntegerinRange 0 255)) (Math|Conversions|ToByte(Integer) (Math|Random|RandomIntegerinRange 0 255)) (Math|Conversions|ToByte(Integer) (Math|Random|RandomIntegerinRange 0 255)) 1))
    (else
      (Utilities|Time|ClearandInvalidateTimerbyHandle (Variables|Default|GetTimerHandle))
      ;[1 1 1] Move to Counter
      (Components|MoveComponentTo _textrender_2 "500.000000,0.000000,0.000000" (.rotation (Transformation|GetRelativeTransform _textrender_2)) true false 2.0 false)
      (Rendering|SetVisibility (Variables|Default|GetTextRender) false false)
      (Variables|/Game/MYContent/Blueprints/BP_PlayFieldConstructror.BP_PlayFieldConstructror_C|SetIsButtonActive (Variables|Default|GetRefToPlayfield) true)
      (Actor|DestroyActor))))

(event EventBeginPlay
  ;[1 1 1] ChangeBubbleColorAndSize
  (bind _returnvalue (Utilities|Time|SetTimerbyFunctionName 0 "MakeTextBigger" (Variables|Default|GetDeltaT) true))
  (Variables|Default|SetTimerHandle _returnvalue))

(fn ConstructionScript
  (bind _textrender (Variables|Default|GetTextRender))
  (Rendering|Components|TextRender|SetXScale _textrender 1.0)
  (Rendering|Components|TextRender|SetYScale _textrender 1.0)
  (bind _outactors (Actor|GetAllActorsOfClass "/Game/MYContent/Blueprints/BP_PlayFieldConstructror.BP_PlayFieldConstructror_C"))
  (Variables|Default|SetRefToPlayfield (Utilities|Array|Get(acopy) _outactors)))