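; BP_Butterfly is a butterfly actor that flits between bubbles on the playfield and rewards freeing it with a combo actor.
; It eases its sphere toward randomly picked bubble coordinates, retrying if it lands without overlapping one.
; When a bubble's overlap ends outside the boss fight, it spawns BP_ButterflyCombo and moves again.
; With no bubbles left, it tumbles downward and destroys itself.
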(event OnComponentEndOverlap(Sphere)
  (params (OverlappedComponent :type Primitive%20Component%20Object%20Reference) (OtherActor :type Actor%20Object%20Reference) (OtherComp :type Primitive%20Component%20Object%20Reference) (OtherBodyIndex :type Integer))
  ;[1 1 1] OnFreeButterfly
  (if (and (Variables|Default|GetIsButterflyOnPosition) (Math|Boolean|NotEqual(Boolean) (Variables|/Game/MYContent/Blueprints/BP_PlayFieldConstructror.BP_PlayFieldConstructror_C|GetIsBossFightStarted (Variables|Default|GetRefToPlayfield)) true))
    (Utilities|Casting|CastToBP_Bubble OtherActor)
    (Variables|Default|SetIsButterflyOnPosition false)
    (Game|SpawnActorfromClass "/Game/MYContent/Blueprints/ART/BP_ButterflyCombo.BP_ButterflyCombo_C" (Math|Transform|MakeTransform "0,0.000000,200.000000" "0,90.000000, 0" "1,1,1") "AlwaysSpawn" 0 0)
    (CallFunction|MoveTORandomBubble)))

(event Custom|MoveTORandomBubble
  (bind _reftoplayfield (Variables|Default|GetRefToPlayfield))
  (bind _paperflipbook (Variables|Default|GetPaperFlipbook))
  (bind _bubblesonplayfield (Variables|/Game/MYContent/Blueprints/BP_PlayFieldConstructror.BP_PlayFieldConstructror_C|GetBubblesOnPlayField _reftoplayfield))
  (bind _returnvalue (Utilities|Array|Length _bubblesonplayfield))
  (bind _returnvalue_2 (- _returnvalue 1))
  (bind _returnvalue_3 (Math|Random|RandomIntegerinRange 0 _returnvalue_2))
  (bind _item (Utilities|Array|Get(acopy) _bubblesonplayfield _returnvalue_3))
  (bind _returnvalue_4 (Transformation|GetActorLocation _item))
  ;[1 1 1] MoveToRandomBubble
  (Audio|Components|Audio|Play _paperflipbook)
  (if (!= _returnvalue 0)
    (Components|MoveComponentTo (Variables|Default|GetSphere) (Math|Vector|MakeVector (.x _returnvalue_4) (+ (.y _returnvalue_4) 1.0) (.z _returnvalue_4)) "0, 0, 0" true false 2.0 false)
    (Audio|Components|Audio|Stop _paperflipbook)
    (Variables|Default|SetIsButterflyOnPosition true)
    (if (< (Utilities|Array|Length (Collision|GetOverlappingActors (Variables|Default|GetSphere) "/Game/MYContent/Blueprints/BP_Bubble.BP_Bubble_C" :!class /Script/Engine.PrimitiveComponent)) 1)
      (CallFunction|MoveTORandomBubble))
    (else
      ;[1 1 1] FinalDEstination
      (CallFunction|FinalDestination))))

(event Custom|FinalDestination
  ;[1 1 1] FinalDEstination
  (Components|MoveComponentTo (Variables|Default|GetSphere) (Math|Vector|MakeVector (Math|Random|RandomFloatinRange -1.5e+02 1.5e+02) 5.0 -1e+03) "180.000000,180.000000,180.000000" false false 4.0 false)
  (Actor|DestroyActor))

(event EventBeginPlay
  ;[1 1 1] BeginPlay
  (CallFunction|MoveTORandomBubble))

(fn ConstructionScript
  (bind _outactors (Actor|GetAllActorsOfClass "/Game/MYContent/Blueprints/BP_PlayFieldConstructror.BP_PlayFieldConstructror_C"))
  (Variables|Default|SetRefToPlayfield (Utilities|Array|Get(acopy) _outactors)))