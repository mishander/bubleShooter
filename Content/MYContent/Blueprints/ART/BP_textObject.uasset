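; BP_textObject is a short-lived floating text actor that flies to a counter and awards match points.
; Construction resets the text scale and caches the first BP_PlayFieldConstructror found in the level.
; On BeginPlay, two chained eased MoveComponentTo calls nudge the TextRender by a random offset, then send it to a fixed counter position.
; It then hides the text, adds PointsPerMatch to the playfield and destroys itself.
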(event EventBeginPlay
  (bind _textrender (Variables|Default|GetTextRender))
  (bind _textrender_2 (Variables|Default|GetTextRender))
  (bind _returnvalue (Transformation|GetWorldTransform _textrender))
  (Components|MoveComponentTo _textrender (Math|Vector|MakeVector (+ (.x (.location _returnvalue)) (Math|Random|RandomFloatinRange 0.0 25.0)) (+ (.y (.location _returnvalue)) (Math|Random|RandomFloatinRange 25.0 75.0)) (+ (.z (.location _returnvalue)) (Math|Random|RandomFloatinRange 0.0 25.0))) (.rotation _returnvalue) true false 0.6 false)
  ;[1 1 1] Move to Counter
  (Components|MoveComponentTo _textrender_2 "-600.000000,0.000000,600.000000" (.rotation (Transformation|GetRelativeTransform _textrender_2)) true false 0.6 false)
  (Rendering|SetVisibility (Variables|Default|GetTextRender) false false)
  (Default|AddPoints (Variables|Default|GetRefToPlayfield) (Math|Conversions|ToInteger(Byte) (Variables|Default|GetPointsPerMatch)))
  (Actor|DestroyActor))

(fn ConstructionScript
  (bind _textrender (Variables|Default|GetTextRender))
  (Rendering|Components|TextRender|SetXScale _textrender 1.0)
  (Rendering|Components|TextRender|SetYScale _textrender 1.0)
  (bind _outactors (Actor|GetAllActorsOfClass "/Game/MYContent/Blueprints/BP_PlayFieldConstructror.BP_PlayFieldConstructror_C"))
  (Variables|Default|SetRefToPlayfield (Utilities|Array|Get(acopy) _outactors)))