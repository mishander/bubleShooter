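; BP_ButterflyCombo is an animated combo text actor that awards bonus points to the playfield and then removes itself.
; A looping timer grows the TextRender toward a target size at constant speed, randomizing its color each step.
; At full size it swaps the text, stops the timer, slides the text away, adds points and destroys itself, sequenced with delays.
; The construction script caches the first BP_PlayFieldConstructror found as the score target.
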(event Custom|MakeTextBigger
  (bind _textrender (Variables|Default|GetTextRender))
  (bind _deltat (Variables|Default|GetDeltaT))
  (bind _worldsize (Variables|/Script/Engine.TextRenderComponent|GetWorldSize _textrender))
  (bind _returnvalue (Math|Interpolation|FInterptoConstant _worldsize 5e+01 _deltat 25.0))
  ;[1 1 1] ChangeBubbleColorAndSize
  (if (< _returnvalue 5e+01)
    (Rendering|Components|TextRender|SetWorldSize _textrender _returnvalue)
    (Rendering|Components|TextRender|SetTextRenderColor (Variables|Default|GetTextRender) (Math|Color|MakeColor (Math|Conversions|ToByte(Integer) (Math|Random|RandomIntegerinRange 0 255)) (Math|Conversions|ToByte(Integer) (Math|Random|RandomIntegerinRange 0 255)) (Math|Conversions|ToByte(Integer) (Math|Random|RandomIntegerinRange 0 255)) 1))
    (else
      (Utilities|FlowControl|Delay 1.0)
      (Rendering|Components|TextRender|SetText (Variables|Default|GetTextRender) (Variables|Default|GetNewVar_0))
      (Utilities|Time|ClearandInvalidateTimerbyHandle (Variables|Default|GetTimerHandle))
      (Utilities|FlowControl|Delay 1.0)
      (Components|MoveComponentTo (Variables|Default|GetTextRender) "-600.000000,0.000000,600.000000" "0.000000,90.000000, 0" false false 1.0 false)
      (Default|AddPoints (Variables|Default|GetRefToPlayfield) 100)
      (Utilities|FlowControl|Delay 0.5)
      (Actor|DestroyActor))))

(event EventBeginPlay
  ;[1 1 1] ChangeBubbleColorAndSize
  (bind _returnvalue (Utilities|Time|SetTimerbyFunctionName 0 "MakeTextBigger" (Variables|Default|GetDeltaT) true))
  (Variables|Default|SetTimerHandle _returnvalue))

(fn ConstructionScript
  (bind _textrender (Variables|Default|GetTextRender))
  (Rendering|Components|TextRender|SetXScale _textrender 1.0)
  (Rendering|Components|TextRender|SetYScale _textrender 1.0)
  (bind _outactors (Actor|GetAllActorsOfClass "/Game/MYContent/Blueprints/BP_PlayFieldConstructror.BP_PlayFieldConstructror_C"))
  (Variables|Default|SetRefToPlayfield (Utilities|Array|Get(acopy) _outactors)))