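; Animated combo text popup actor that grows, flashes random colours and celebrates with explosions before destroying itself.
; A looping timer interpolates the text's world size up while randomizing its colour, and a second timer spawns bubble explosion effects around it.
; At full size it activates five particle systems tinted in the construction script, moves the text away, then destroys the actor.
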(event Custom|MakeTextBigger
  (bind _textrender (Variables|Default|GetTextRender))
  (bind _deltat (Variables|Default|GetDeltaT))
  (bind _worldsize (Variables|/Script/Engine.TextRenderComponent|GetWorldSize _textrender))
  (bind _returnvalue (Math|Interpolation|FInterptoConstant _worldsize 1e+02 _deltat 66.0))
  ;[1 1 1] ChangeBubbleColorAndSize
  (if (< _returnvalue 1e+02)
    (Rendering|Components|TextRender|SetWorldSize _textrender _returnvalue)
    (Rendering|Components|TextRender|SetTextRenderColor (Variables|Default|GetTextRender) (Math|Color|MakeColor (Math|Conversions|ToByte(Integer) (Math|Random|RandomIntegerinRange 0 255)) (Math|Conversions|ToByte(Integer) (Math|Random|RandomIntegerinRange 0 255)) (Math|Conversions|ToByte(Integer) (Math|Random|RandomIntegerinRange 0 255)) 1))
    (else
      (Utilities|Time|ClearandInvalidateTimerbyHandle (Variables|Default|GetTimerHandle))
      (Utilities|FlowControl|Delay 1.0)
      (Components|Activation|SetActive (Variables|Default|GetParticleSystem) true false)
      (Components|Activation|SetActive (Variables|Default|GetParticleSystem1) true false)
      (Components|Activation|SetActive (Variables|Default|GetParticleSystem2) true false)
      (Components|Activation|SetActive (Variables|Default|GetParticleSystem3) true false)
      (Components|Activation|SetActive (Variables|Default|GetParticleSystem4) true false)
      (Components|MoveComponentTo (Variables|Default|GetTextRender) "-600.000000,0.000000,600.000000" "0.000000,90.000000, 0" false false 1.0 false)
      (Utilities|FlowControl|Delay 0.5)
      (Actor|DestroyActor))))

(event Custom|SpawnRandomExplosion
  (bind _textrender (Variables|Default|GetTextRender))
  (bind _returnvalue (Transformation|GetWorldLocation _textrender))
  (Game|SpawnActorfromClass "/Game/MYContent/Blueprints/Effects/BP_BubbleExplosionEffect.BP_BubbleExplosionEffect_C" (Math|Transform|MakeTransform (Math|Vector|MakeVector (+ (.x _returnvalue) (Math|Random|RandomFloatinRange -1.5e+02 1.5e+02)) (+ (.y _returnvalue) -5e+01) (+ (.z _returnvalue) (Math|Random|RandomFloatinRange -3e+01 3e+01))) "0, 0, 0" "0.500000,0.500000,0.500000") "AlwaysSpawn" 0 0))

(event EventBeginPlay
  ;[1 1 1] ChangeBubbleColorAndSize
  (Utilities|Time|SetTimerbyFunctionName 0 "SpawnRandomExplosion" 0.75 true)
  (bind _returnvalue (Utilities|Time|SetTimerbyFunctionName 0 "MakeTextBigger" (Variables|Default|GetDeltaT) true))
  (Variables|Default|SetTimerHandle _returnvalue))

(fn ConstructionScript
  (bind _textrender (Variables|Default|GetTextRender))
  (Rendering|Components|TextRender|SetXScale _textrender 1.0)
  (Rendering|Components|TextRender|SetYScale _textrender 1.0)
  (bind _outactors (Actor|GetAllActorsOfClass "/Game/MYContent/Blueprints/BP_PlayFieldConstructror.BP_PlayFieldConstructror_C"))
  (Variables|Default|SetRefToPlayfield (Utilities|Array|Get(acopy) _outactors))
  (Effects|Components|ParticleSystem|SetColorParameter (Variables|Default|GetParticleSystem) "PassColor" (Utilities|Struct|MakeLinearColor 1.0 0.0 0.0 1.0))
  (Effects|Components|ParticleSystem|SetColorParameter (Variables|Default|GetParticleSystem1) "PassColor" (Utilities|Struct|MakeLinearColor 0.0 1.0 0.0 1.0))
  (Effects|Components|ParticleSystem|SetColorParameter (Variables|Default|GetParticleSystem2) "PassColor" (Utilities|Struct|MakeLinearColor 0.0 0.0 1.0 1.0))
  (Effects|Components|ParticleSystem|SetColorParameter (Variables|Default|GetParticleSystem3) "PassColor" (Utilities|Struct|MakeLinearColor 0.7 1.0 0.0 1.0))
  (Effects|Components|ParticleSystem|SetColorParameter (Variables|Default|GetParticleSystem4) "PassColor" (Utilities|Struct|MakeLinearColor 0.98 0.33 0.0 1.0)))