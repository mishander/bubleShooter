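; BP_Minion2 is a minion actor with a Sphere component and two particle components, PRight and PLeft, which its construction script tints blue through the PassColor parameter.
; Each tick, it flips the small relative Y offset of both particle components based on the sign of the actor's world X position.
; MoveActorToLocationPerTime moves the Sphere to a given X/Z target over a set time, with fixed Y and rotation.
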(event Custom|MoveActorToLocationPerTime
  (params (DestinationX :type Float%20%28single-precision%29) (DestinationZ :type Float%20%28single-precision%29) (Time :type Float%20%28single-precision%29))
  (Components|MoveComponentTo (Variables|Default|GetSphere) (Math|Vector|MakeVector DestinationX -2.0 DestinationZ) "0.000000, 0,180.000000" false false Time false))

(event EventTick
  (params (DeltaSeconds :type Float%20%28single-precision%29))
  (if (>= (.x (Transformation|GetActorLocation)) 0.0)
    (Transformation|SetRelativeLocation (Variables|Default|GetP_Right) (Math|Vector|MakeVector 17.0 2.0 -66.0) false false)
    (Transformation|SetRelativeLocation (Variables|Default|GetP_Left) (Math|Vector|MakeVector -16.0 2.0 -66.0) false false)
    (else
      (Transformation|SetRelativeLocation (Variables|Default|GetP_Right) (Math|Vector|MakeVector 17.0 -2.0 -66.0) false false)
      (Transformation|SetRelativeLocation (Variables|Default|GetP_Left) (Math|Vector|MakeVector -16.0 -2.0 -66.0) false false))))

(fn ConstructionScript
  (Effects|Components|ParticleSystem|SetColorParameter (Variables|Default|GetP_Right) "PassColor" (Utilities|Struct|MakeLinearColor 0.0 0.5 1.0 1.0))
  (Effects|Components|ParticleSystem|SetColorParameter (Variables|Default|GetP_Left) "PassColor" (Utilities|Struct|MakeLinearColor 0.0 0.5 1.0 1.0)))