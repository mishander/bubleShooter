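; BP_Sun is a temporary sun hazard that grows over time and pops bubbles it touches.
; A looping timer started on BeginPlay eases the Sphere's world scale toward a fixed maximum at constant speed, using DeltaTime as both interval and interpolation step.
; Any BP_Bubble that begins overlapping the Sphere is told to self-destruct.
; The actor destroys itself after SunLifeTime elapses.
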(event OnComponentBeginOverlap(Sphere)
  (params (OverlappedComponent :type Primitive%20Component%20Object%20Reference) (OtherActor :type Actor%20Object%20Reference) (OtherComp :type Primitive%20Component%20Object%20Reference) (OtherBodyIndex :type Integer) (bFromSweep :type Boolean) (SweepResult :type Hit%20Result%20Structure%20%28by%20ref%29))
  ;[1 1 1] Overlap
  (bind _asbp_bubble (Utilities|Casting|CastToBP_Bubble OtherActor))
  (Default|SelfDestruction _asbp_bubble))

(event Custom|IncreaseSun
  ;[1 1 1] IncreaseSun
  (Transformation|SetWorldScale3D (Variables|Default|GetSphere) (Math|Interpolation|VInterptoConstant (Transformation|GetWorldScale (Variables|Default|GetSphere)) "5.000000,5.000000,5.000000" (Variables|Default|GetDeltaTime) 0.5)))

(event EventBeginPlay
  ;[1 1 1] BeginPlay
  (Utilities|Time|SetTimerbyFunctionName 0 "IncreaseSun" (Variables|Default|GetDeltaTime) true)
  (Utilities|FlowControl|Delay (Variables|Default|GetSunLifeTime))
  (Actor|DestroyActor))

(fn ConstructionScript)