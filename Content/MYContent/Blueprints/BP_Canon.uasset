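; BP_Canon is the player's bubble-shooter cannon, which rotates to follow the mouse cursor and shows a predicted shot path.
; Each tick it sphere-traces along the aim, adds a mirrored second trace when hitting BlackCorners, and draws both segments with two beams.
; A cannon state gates shooting and swapping, delegated to the playfield, which also spawns the next bubble after delays.
; Number keys trigger boss-fight, attack, minion-spawn and print shortcuts.
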(event Custom|BuildBeam
  (bind _experimentalbeam (Variables|Default|GetExperimentalBeam))
  (bind _experimentalbeam2 (Variables|Default|GetExperimentalBeam2))
  (bind _point1x (Variables|Default|GetPoint1X))
  (bind _point1z (Variables|Default|GetPoint1Z))
  (bind _cube (Variables|Default|GetCube))
  (bind _returnvalue (Transformation|GetWorldTransform _cube))
  ;[1 1 1] BuildBeam
  (Class|ParticleSystemComponent|SetBeamSourcePoint _experimentalbeam 0 (Math|Vector|MakeVector (.x (.location _returnvalue)) -2.0 (.z (.location _returnvalue))))
  (Class|ParticleSystemComponent|SetBeamTargetPoint _experimentalbeam 0 (Math|Vector|MakeVector _point1x -2.0 _point1z))
  (Class|ParticleSystemComponent|SetBeamSourcePoint _experimentalbeam2 0 (Math|Vector|MakeVector _point1x 0.0 _point1z))
  (Class|ParticleSystemComponent|SetBeamTargetPoint _experimentalbeam2 0 (Math|Vector|MakeVector (Variables|Default|GetPoint2X) 0.0 (Variables|Default|GetPoint2Z)))
  (CallFunction|UpdateCannonPosition))

(event Custom|ChangeHealth
  (params (ChangeHEalthParam :type Float%20%28single-precision%29))
  ;[1 1 1] ChangeHealth
  (Variables|Default|SetHealth (+ (Variables|Default|GetHealth) ChangeHEalthParam)))

(event Custom|UpdateCannonPosition
  (bind _returnvalue (Game|GetPlayerController 0))
  (bind (_locationx _locationy) (Game|Player|GetMousePosition _returnvalue))
  ;[1 1 1] Mouse move on cursor
  (if (<= _locationy (Variables|Default|GetWhereWeshouldIgnoreCursor))
    (Transformation|SetWorldRotation (Variables|Default|GetCube) (Math|Interpolation|RInterpTo (Transformation|GetActorRotation) (Math|Rotator|MakeRotator 1.8e+02 (+ (.Yaw (Math|Rotator|BreakRotator (Math|Rotator|FindLookatRotation (Math|Conversions|ToVector(Vector2D) (.ScreenLocation (Class|PlayerController|ProjectWorldLocationtoScreen (Game|GetPlayerController 0) (Transformation|GetActorLocation) false))) (Math|Conversions|ToVector(Vector2D) (Math|Vector2D|MakeVector2D _locationx _locationy))))) 2.7e+02) 1.8e+02) 1.0 1.0) false false))
  ;[1 1 1] EventTick
  (if (Utilities|Enum|Equal(Enum) (Variables|Default|GetCannonState) "NewEnumerator1")
    (Utilities|FlowControl|Delay 0.2)
    (Default|SpawnRandomBubbleforShooting (Variables|Default|GetPlayfield))
    (Variables|Default|SetCannonState "NewEnumerator0")))

(event EventTick
  (params (DeltaSeconds :type Float%20%28single-precision%29))
  (bind _cube (Variables|Default|GetCube))
  (bind _cube_2 (Variables|Default|GetCube))
  (bind _returnvalue (Transformation|GetWorldTransform _cube))
  (bind _returnvalue_2 (Transformation|GetWorldTransform _cube_2))
  (bind _returnvalue_3 (- 9e+01 (.pitch (.rotation _returnvalue))))
  (bind _returnvalue_4 (+ (.pitch (.rotation _returnvalue_2)) 9e+01))
  (bind _returnvalue_5 (Math|Float|Absolute(Float) _returnvalue_3))
  (bind _returnvalue_6 (Math|Float|Absolute(Float) _returnvalue_4))
  ;[1 1 1] EventTick
  ;[1 1 1] GetPointsForCannonAim
  (bind _outhit (Collision|SphereTraceForObjects (Math|Vector|MakeVector (.x (.location _returnvalue_2)) (.y (.location _returnvalue_2)) (.z (.location _returnvalue_2))) (Math|Vector|MakeVector (|(x+(2000*cosAlpha)) (.x (.location _returnvalue_2)) (Math|Trig|Cos(Degrees) _returnvalue_6)) 0.0 (|(z+(2000*sinAlpha)) (.z (.location _returnvalue_2)) (Math|Trig|Sin(Degrees) _returnvalue_6))) 2e+01 (Utilities|Array|MakeArray "ObjectTypeQuery2") true 0 "None"))
  (Variables|Default|SetPoint1X (.x (.Location (Collision|BreakHitResult _outhit))))
  (Variables|Default|SetPoint1Z (.z (.Location (Collision|BreakHitResult _outhit))))
  (Utilities|Casting|CastToBlackCorners (.HitActor (Collision|BreakHitResult _outhit))
    (:then
      (bind _outhit_2 (Collision|SphereTraceForObjects (Math|Vector|MakeVector (|(x-(x2/x)) (.x (.Location (Collision|BreakHitResult _outhit))) (Math|Float|Absolute(Float) (.x (.Location (Collision|BreakHitResult _outhit))))) (.y (.Location (Collision|BreakHitResult _outhit))) (.z (.Location (Collision|BreakHitResult _outhit)))) (Math|Vector|MakeVector (|(x+(2000*cosAlpha)) (|(x-(x2/x)) (.x (.Location (Collision|BreakHitResult _outhit))) (Math|Float|Absolute(Float) (.x (.Location (Collision|BreakHitResult _outhit))))) (Math|Trig|Cos(Degrees) _returnvalue_5)) 0.0 (|(z+(2000*sinAlpha)) (.z (.ImpactPoint (Collision|BreakHitResult _outhit))) (Math|Trig|Sin(Degrees) _returnvalue_5))) 2e+01 (Utilities|Array|MakeArray "ObjectTypeQuery2") true 0 "None" true "(R=0.055220,G=0.021443,B=1.000000,A=1.000000)" "(R=1.000000,G=0.901327,B=0.068713,A=1.000000)"))
      (Variables|Default|SetPoint2X (.x (.location _outhit_2)))
      (Variables|Default|SetPoint2Z (.z (.location _outhit_2))))
    (:CastFailed
      (Variables|Default|SetPoint2X (Variables|Default|GetPoint1X))
      (Variables|Default|SetPoint2Z (Variables|Default|GetPoint1Z))))
  (CallFunction|BuildBeam))

(event Input|ActionEvents|InputActionShoot
  (params (Key :type Key%20Structure :default "AnyKey"))
  ;[1 1 1] Shooting
  (:Pressed
    (if (Utilities|Enum|Equal(Enum) (Variables|Default|GetCannonState) "NewEnumerator0")
      (Default|LaunchBubble (Variables|Default|GetPlayfield))
      (Variables|Default|SetCannonState "NewEnumerator2")
      (Utilities|FlowControl|Delay 0.4)
      (Variables|Default|SetCannonState "NewEnumerator1"))))

(event Input|ActionEvents|InputActionSwitchBubbles
  (params (Key :type Key%20Structure :default "AnyKey"))
  ;[1 1 1] SwitchBetweenCannonAndColar
  (:Pressed
    (if (Utilities|Enum|Equal(Enum) (Variables|Default|GetCannonState) "NewEnumerator0")
      (Default|SwapPlaces (Variables|Default|GetPlayfield)))))

(event Input|KeyboardEvents|1
  (params (Key :type Key%20Structure :default "AnyKey"))
  (:Pressed
    (bind _outactors (Actor|GetAllActorsOfClass "/Game/MYContent/Blueprints/BP_BOSS.BP_BOSS_C"))
    (Default|AttackBot (Utilities|Array|Get(acopy) _outactors))))

(event Input|KeyboardEvents|9
  (params (Key :type Key%20Structure :default "AnyKey"))
  (:Pressed
    (bind _outactors (Actor|GetAllActorsOfClass "/Game/MYContent/Blueprints/BP_BOSS.BP_BOSS_C"))
    (for _array_element (Actor|GetAttachedActors (Utilities|Array|Get(acopy) _outactors))
      (Development|PrintString (Utilities|GetDisplayName _array_element)))))

(event Input|KeyboardEvents|4
  (params (Key :type Key%20Structure :default "AnyKey"))
  (:Pressed
    (Default|StartBossFight (Variables|Default|GetPlayfield))))

(event Input|KeyboardEvents|2
  (params (Key :type Key%20Structure :default "AnyKey"))
  (:Pressed
    (Game|SpawnActorfromClass "/Game/MYContent/Blueprints/BP_Minion2.BP_Minion2_C" (Math|Transform|MakeTransform "0, 0,200.000000" "0, 0, 0" "0.500000,0.500000,0.500000") "Undefined" 0 0)))

(fn ConstructionScript
  (bind _outactors (Actor|GetAllActorsOfClass "/Game/MYContent/Blueprints/BP_PlayFieldConstructror.BP_PlayFieldConstructror_C"))
  (Variables|Default|SetPlayfield (Utilities|Array|Get(acopy) _outactors))
  (bind _outactors_2 (Actor|GetAllActorsOfClass "/Game/MYContent/Blueprints/InvisibleSceneRoot.InvisibleSceneRoot_C"))
  (Variables|Default|SetInvisibleSceneRoot (Utilities|Array|Get(acopy) _outactors_2))
  (bind _outactors_3 (Actor|GetAllActorsOfClass "/Game/MYContent/Blueprints/BP_RocketManager.BP_RocketManager_C"))
  (Variables|Default|SetRocketManager (Utilities|Array|Get(acopy) _outactors_3)))