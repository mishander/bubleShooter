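; BP_Bubble is the colored bubble actor for a bubble shooter, serving as projectile and field piece.
; On bouncing off another bubble, it snaps into one of six hex slots using impact side and slope, then joins the playfield.
; It recursively flags matching-color neighbours before the Playfield removes matches and unlinked bubbles and checks for line respawn.
; Helper events handle sprite tint, colored trail, and delayed destruction with score text.
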(event OnProjectileBounce(ProjectileMovement)
  (params (ImpactResult :type Hit%20Result%20Structure%20%28by%20ref%29) (ImpactVelocity :type Vector%20%28by%20ref%29 :default "0, 0, 0"))
  ;[1 1 1] ImpactOfShootAndBubble
  (bind _asbp_bubble (Utilities|Casting|CastToBP_Bubble (.hitactor ImpactResult)))
  (bind _output_get (Variables|Default|SetPlaceOfImpact (.location ImpactResult)))
  (if (Math|Boolean|ANDBoolean (>= (.x _output_get) (.x (.location (Transformation|GetActorTransform _asbp_bubble)))) (>= (.z _output_get) (.z (.location (Transformation|GetActorTransform _asbp_bubble)))) (< (Math|Float|Absolute(Float) (|((x2-x1)/(z2-z1)) (.x _output_get) (.x (.location (Transformation|GetActorTransform _asbp_bubble))) (.z _output_get) (.z (.location (Transformation|GetActorTransform _asbp_bubble))))) 2.0))
    (Variables|Default|SetDisplacementOfShootOnAttachX 22.0)
    (Variables|Default|SetDisplacementOfShootOnAttachZ 38.0)
    (CallFunction|StopProjectile :!label _label)
    (CallFunction|StickProjectiletoField)
    (CallFunction|CheckBubblesColor)
    (Utilities|FlowControl|Delay 0.1)
    (Default|KillBubblesOftheSameColor (Variables|Default|GetPlayfield))
    (Default|CheckRooted (Variables|Default|GetPlayfield))
    (Default|KillUnlinkedBubbles (Variables|Default|GetPlayfield))
    (Default|CheckifWeNeedtoRespawnLine (Variables|Default|GetPlayfield))
    (elif (and (>= (.x _output_get) (.x (.location (Transformation|GetActorTransform _asbp_bubble)))) (>= (Math|Float|Absolute(Float) (|((x2-x1)/(z2-z1)) (.x _output_get) (.x (.location (Transformation|GetActorTransform _asbp_bubble))) (.z _output_get) (.z (.location (Transformation|GetActorTransform _asbp_bubble))))) 2.0))
      (Variables|Default|SetDisplacementOfShootOnAttachX 44.0)
      (Variables|Default|SetDisplacementOfShootOnAttachZ 0.0)
      (goto _label)
      (elif (Math|Boolean|ANDBoolean (>= (.x _output_get) (.x (.location (Transformation|GetActorTransform _asbp_bubble)))) (< (.z _output_get) (.z (.location (Transformation|GetActorTransform _asbp_bubble)))) (< (Math|Float|Absolute(Float) (|((x2-x1)/(z2-z1)) (.x _output_get) (.x (.location (Transformation|GetActorTransform _asbp_bubble))) (.z _output_get) (.z (.location (Transformation|GetActorTransform _asbp_bubble))))) 2.0))
        (Variables|Default|SetDisplacementOfShootOnAttachX 22.0)
        (Variables|Default|SetDisplacementOfShootOnAttachZ -38.0)
        (goto _label)
        (elif (Math|Boolean|ANDBoolean (< (.x _output_get) (.x (.location (Transformation|GetActorTransform _asbp_bubble)))) (< (.z _output_get) (.z (.location (Transformation|GetActorTransform _asbp_bubble)))) (< (Math|Float|Absolute(Float) (|((x2-x1)/(z2-z1)) (.x _output_get) (.x (.location (Transformation|GetActorTransform _asbp_bubble))) (.z _output_get) (.z (.location (Transformation|GetActorTransform _asbp_bubble))))) 2.0))
          (Variables|Default|SetDisplacementOfShootOnAttachX -22.0)
          (Variables|Default|SetDisplacementOfShootOnAttachZ -38.0)
          (goto _label)
          (elif (and (>= (Math|Float|Absolute(Float) (|((x2-x1)/(z2-z1)) (.x _output_get) (.x (.location (Transformation|GetActorTransform _asbp_bubble))) (.z _output_get) (.z (.location (Transformation|GetActorTransform _asbp_bubble))))) 2.0) (< (.x _output_get) (.x (.location (Transformation|GetActorTransform _asbp_bubble)))))
            (Variables|Default|SetDisplacementOfShootOnAttachX -44.0)
            (Variables|Default|SetDisplacementOfShootOnAttachZ 0.0)
            (goto _label)
            (elif (Math|Boolean|ANDBoolean (>= (.z _output_get) (.z (.location (Transformation|GetActorTransform _asbp_bubble)))) (< (.x _output_get) (.x (.location (Transformation|GetActorTransform _asbp_bubble)))) (< (Math|Float|Absolute(Float) (|((x2-x1)/(z2-z1)) (.x _output_get) (.x (.location (Transformation|GetActorTransform _asbp_bubble))) (.z _output_get) (.z (.location (Transformation|GetActorTransform _asbp_bubble))))) 2.0))
              (Variables|Default|SetDisplacementOfShootOnAttachX -22.0)
              (Variables|Default|SetDisplacementOfShootOnAttachZ 38.0)
              (goto _label))))))))

(event Custom|ActivateTrace
  (bind _trace (Variables|Default|GetTrace))
  ;[1 1 1] ActivateTrace
  (Components|Activation|SetActive _trace true false)
  (Effects|Components|ParticleSystem|SetColorParameter _trace "PassColor" (Variables|/Script/Paper2D.PaperSpriteComponent|GetSpriteColor (Variables|Default|GetPaperSprite))))

(event Custom|DeactivateTrace
  ;[1 1 1] DeactivateTrace
  (Components|Activation|SetActive (Variables|Default|GetTrace) false false))

(event Custom|StopProjectile
  ;[1 1 1] StopProjectile
  (Components|Movement|StopMovementImmediately (Variables|Default|GetProjectileMovement)))

(event Custom|DelayedSelfDestruction
  ;[1 1 1] DelayedSelfDestruction
  (Utilities|FlowControl|Delay 0.7)
  (if (Variables|Default|GetThisBubbleSpecial)
    ;;[1 1 1] DeathOfSpecialBubble
    (Default|RespawnScoreText (Variables|Default|GetPlayfield) self "?")
    (Actor|DestroyActor)
    (else
      (Default|RespawnScoreText (Variables|Default|GetPlayfield) self "25")
      (Actor|DestroyActor))))

(event Custom|ChangebubbleColor
  (bind _papersprite (Variables|Default|GetPaperSprite))
  ;[1 1 1] ChangeBubbleColor
  (switch Utilities|FlowControl|Switch|SwitchonEnumColors (Variables|Default|GetPassedColors)
    (:NewEnumerator0
      (Sprite|SetSpriteColor _papersprite (Utilities|Struct|MakeLinearColor 1.0 0.0 0.0 1.0)))
    (:NewEnumerator1
      (Sprite|SetSpriteColor _papersprite (Utilities|Struct|MakeLinearColor 0.0 0.5 1.0 1.0)))
    (:NewEnumerator2
      (Sprite|SetSpriteColor _papersprite (Utilities|Struct|MakeLinearColor 0.1 1.0 0.0 1.0)))
    (:NewEnumerator3
      (Sprite|SetSpriteColor _papersprite (Utilities|Struct|MakeLinearColor 0.97 1.0 0.0 1.0)))
    (:NewEnumerator4
      (Sprite|SetSpriteColor _papersprite (Utilities|Struct|MakeLinearColor 0.98 0.33 0.0 1.0)))
    (:NewEnumerator5
      (Sprite|SetSpriteColor _papersprite (Utilities|Struct|MakeLinearColor 1.0 0.0 0.0 1.0)))
    (:NewEnumerator6
      (Sprite|SetSpriteColor _papersprite (Utilities|Struct|MakeLinearColor 1.0 1.0 1.0 0.0)))))

(event Custom|CheckBubblesColor
  ;[1 1 1] CheckBubblesColor
  (for _array_element (Variables|Default|GetBubbleNeighbours)
    (if (Utilities|Enum|Equal(Enum) (Variables|Default|GetPassedColors) (Variables|BP_Bubble_C|GetPassedColors _array_element))
      (Variables|Default|SetProjectileNeedToBeRemoved true)
      (if (Math|Boolean|NotEqual(Boolean) (Variables|BP_Bubble_C|GetProjectileNeedToBeRemoved _array_element) true)
        (Variables|BP_Bubble_C|SetProjectileNeedToBeRemoved _array_element true)
        (CallFunction|CheckBubblesColor _array_element)))))

(event Custom|StickProjectileToField
  ;[1 1 1] StickProjectileToField
  (Transformation|SetActorLocation (Math|Vector|MakeVector (+ (Variables|Default|GetDisplacementOfShootOnAttachX) (.x (.location (Transformation|GetActorTransform (stale OnProjectileBounce(ProjectileMovement) _asbp_bubble))))) (.y (.location (Transformation|GetActorTransform (stale OnProjectileBounce(ProjectileMovement) _asbp_bubble)))) (+ (Variables|Default|GetDisplacementOfShootOnAttachZ) (.z (.location (Transformation|GetActorTransform (stale OnProjectileBounce(ProjectileMovement) _asbp_bubble)))))) false false)
  (Default|AddtoPlayFieldArray (Variables|Default|GetPlayfield) self)
  (Transformation|AttachActorToActor (Variables|Default|GetInvisibleSceneRoot) "None" "KeepWorld" "KeepWorld" "KeepWorld" false)
  (CallFunction|DeactivateTrace))

(fn ConstructionScript
  (bind _outactors (Actor|GetAllActorsOfClass "/Game/MYContent/Blueprints/BP_PlayFieldConstructror.BP_PlayFieldConstructror_C"))
  (Variables|Default|SetPlayfield (Utilities|Array|Get(acopy) _outactors))
  (bind _outactors_2 (Actor|GetAllActorsOfClass "/Game/MYContent/Blueprints/InvisibleSceneRoot.InvisibleSceneRoot_C"))
  (Variables|Default|SetInvisibleSceneRoot (Utilities|Array|Get(acopy) _outactors_2)))