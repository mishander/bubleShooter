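; Boss actor for a 2D sprite fight, damaged by BP_Bubble hits with a red flash and destroyed at zero health.
; Timers fill cooldowns polled on Tick, alternately spawning one or two minions that each take six bubbles from the boss's ring shield.
; An empty shield triggers a recharge with reduced damage taken, then respawns the ring.
; Health thresholds make BossFightManager call bombers, then start periodic sun-marker launches to random preset positions.
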(event OnComponentHit(Sphere)
  (params (HitComponent :type Primitive%20Component%20Object%20Reference) (OtherActor :type Actor%20Object%20Reference) (OtherComp :type Primitive%20Component%20Object%20Reference) (NormalImpulse :type Vector :default "0, 0, 0") (Hit :type Hit%20Result%20Structure%20%28by%20ref%29))
  (bind _papersprite (Variables|Default|GetPaperSprite))
  ;[1 1 1] HitByBubble
  (bind _asbp_bubble (Utilities|Casting|CastToBP_Bubble OtherActor))
  (CallFunction|ChangeHealth (Variables|Default|GetDamageOnHitByBubble))
  (Default|SelfDestruction _asbp_bubble)
  ;[1 1 1] EffectOfRedHit
  (Timeline|Timeline_0 PlayFromStart
    (:Update
      (Sprite|SetSpriteColor _papersprite (Class|KismetMathLibrary|CInterpto (Variables|/Script/Paper2D.PaperSpriteComponent|GetSpriteColor _papersprite) (Utilities|Struct|MakeLinearColor 1.0 0.0 0.0 1.0) 0.3 1.0)))
    (:Finished
      (Sprite|SetSpriteColor _papersprite (Utilities|Struct|MakeLinearColor 1.0 1.0 1.0 1.0)))))

(event Custom|MoveActorToLocation
  (params (DestinationX :type Float%20%28single-precision%29) (DestinationZ :type Float%20%28single-precision%29) (Time :type Float%20%28single-precision%29))
  ;[1 1 1] MoveToLocation
  (Components|MoveComponentTo (Variables|Default|GetPaperSprite) (Math|Vector|MakeVector DestinationX 0.0 DestinationZ) "0.000000, 0,0.000000" false true Time false)
  (Default|BossonPosition (Variables|Default|GetRefToBossManager)))

(event Custom|SetUpTimersForAbilities
  ;[1 1 1] SetUpTimersForAbilities
  (bind _returnvalue (Utilities|Time|SetTimerbyFunctionName 0 "AddMinion2Timer" 1.0 true))
  (Variables|Default|SetMinionCooldownHandle _returnvalue))

(event Custom|AddMinion2Timer
  ;[1 1 1] AddMinion2Timer
  (Variables|Default|SetMinion2RespawnCooldown (+ (Variables|Default|GetMinion2RespawnCooldown) 0.07)))

(event Custom|SpawnSunMarkerAndSEndONposition
  (params (X :type Float%20%28single-precision%29) (Z :type Float%20%28single-precision%29))
  (bind _papersprite (Variables|Default|GetPaperSprite))
  (bind _returnvalue (Transformation|GetWorldLocation _papersprite))
  ;[1 1 1] SpawnSunMarkerAndSEndONposition
  (bind _returnvalue_2 (Game|SpawnActorfromClass "/Game/MYContent/Blueprints/BP_SunMarker.BP_SunMarker_C" (Math|Transform|MakeTransform (Math|Vector|MakeVector (.x _returnvalue) (- (.y _returnvalue) 1.0) (.z _returnvalue)) "0, 0,180.000000" "1,1,1") "AlwaysSpawn" 0 0))
  (Default|MoveActortoLocationPerTime _returnvalue_2 X Z 1.0))

(event Custom|StartChargingShield
  (bind _papersprite (Variables|Default|GetPaperSprite))
  (bind _returnvalue (Transformation|GetWorldLocation _papersprite))
  (bind _returnvalue_2 (+ (.y _returnvalue) 1.0))
  ;[1 1 1] StartChargingShield
  (Variables|Default|SetDamageOnHitByBubble -0.005)
  (Variables|Default|SetBossNotRecharging false)
  (Effects|SpawnEmitteratLocation "/Game/MYContent/Blueprints/Effects/P_UFOCharging.P_UFOCharging" (Math|Vector|MakeVector (.x _returnvalue) _returnvalue_2 (.z _returnvalue)))
  (Timeline|Timeline_1 PlayFromStart
    (:Finished
      (Effects|SpawnEmitteratLocation "/Game/MYContent/Blueprints/Effects/P_UFOReady.P_UFOReady" (Math|Vector|MakeVector (.x _returnvalue) _returnvalue_2 (.z _returnvalue)))
      (Timeline|Timeline_2 PlayFromStart
        (:Finished
          (CallFunction|RaiseShield)
          (Variables|Default|SetBossNotRecharging true)
          (Variables|Default|SetDamageOnHitByBubble -0.025))))))

(event Custom|RaiseShield
  (bind _sphere (Variables|Default|GetSphere))
  (bind _returnvalue (Transformation|GetWorldLocation _sphere))
  ;[1 1 1] RaiseShield
  (for _index (range 0 47)
    (bind _returnvalue_2 (Game|SpawnActorfromClass "/Game/MYContent/Blueprints/BP_BossBubble.BP_BossBubble_C" (Math|Transform|MakeTransform (Math|Vector|MakeVector (+ (.x _returnvalue) (* (Math|Trig|Sin(Degrees) (* _index 7.5)) 4e+02)) 1.0 (+ (.z _returnvalue) (* (Math|Trig|Cos(Degrees) (* _index 7.5)) 4e+02))) "0, 0, 0" "1,1,1") "AlwaysSpawn" 0 0))
    (Transformation|AttachActorToActor _returnvalue_2 self "None" "KeepWorld" "KeepWorld" "KeepWorld" false)
    (Utilities|Array|Add (Variables|Default|GetBossShieldBubble) _returnvalue_2)))

(event Custom|SpawnBot
  (params (z :type Float%20%28single-precision%29) (X :type Float%20%28single-precision%29))
  ;[1 1 1] SpawnBot
  (bind _returnvalue (Game|SpawnActorfromClass "/Game/MYContent/Blueprints/BP_Minion2.BP_Minion2_C" (Math|Transform|MakeTransform (Math|Vector|MakeVector 0.0 -2.0 7e+02) "0.000000,0.000000,180.000000" "0.500000,0.500000,0.500000") "AlwaysSpawn" 0 0))
  (Default|MoveActortoLocationPerTime _returnvalue (+ (Variables|Default|GetMinion2X) -3.0) (+ (Variables|Default|GetMinion2Z) -3.0) 3.0))

(event Custom|BossDeath
  ;[1 1 1] BossDeath
  (Actor|DestroyActor))

(event Custom|SunGeneratingPhase
  ;[1 1 1] SunGeneratingPhase
  (Utilities|Time|SetTimerbyFunctionName 0 "SunCooldown" 1.0 true))

(event Custom|ChangeHealth
  (params (DeltaHealth :type Float%20%28single-precision%29))
  ;[1 1 1] ChangeHealth
  (Variables|Default|SetHealth (+ (Variables|Default|GetHealth) DeltaHealth)))

(event Custom|StartBotAttack
  (params (RefToAttackingBot :type BP%20Minion%202%20Object%20Reference))
  (bind _reftocannon (Variables|Default|GetRefToCannon))
  (bind _returnvalue (Transformation|GetActorLocation _reftocannon))
  ;[1 1 1] StartBotAttack
  (Default|MoveActortoLocationPerTime RefToAttackingBot (.x _returnvalue) (.z _returnvalue) 15.0))

(event Custom|2AttackBotSequence
  ;[1 1 1] 2AttackBotSequence
  (Variables|Default|SetMinion2X -2e+02)
  (Variables|Default|SetMinion2Z 3.6e+02)
  (CallFunction|MakeAttackBotBubbles)
  (Variables|Default|SetMinion2X 2.2e+02)
  (Variables|Default|SetMinion2Z 3.6e+02)
  (CallFunction|MakeAttackBotBubbles))

(event Custom|1AttackBotSequence
  ;[1 1 1] 1AttackBotSequence
  (Variables|Default|SetMinion2X 0.0)
  (Variables|Default|SetMinion2Z 3.6e+02)
  (CallFunction|MakeAttackBotBubbles))

(event Custom|SunCooldown
  ;[1 1 1] SunCooldown
  (Variables|Default|SetSunREspawnCooldown (+ (Variables|Default|GetSunREspawnCooldown) 0.2)))

(event Custom|MakeAttackBotBubbles
  (bind _bossshieldbubble (Variables|Default|GetBossShieldBubble))
  (bind _returnvalue (Utilities|Array|Length _bossshieldbubble))
  ;[1 1 1] MakeAttackBotBubblesAndBot
  (if (!= _returnvalue 0)
    (CallFunction|SpawnBot (Variables|Default|GetMinion2Z) (Variables|Default|GetMinion2X))
    (for _index (range 0 5)
      (bind _output_get (Variables|Default|SetArrayIndex (Math|Random|RandomIntegerinRange 0 (- _returnvalue 1))))
      (switch int _index
        (:0
          (Variables|Default|SetDissplacementX 22.0)
          (Variables|Default|SetDissplacementZ 38.0))
        (:1
          (Variables|Default|SetDissplacementX 44.0)
          (Variables|Default|SetDissplacementZ 0.0))
        (:2
          (Variables|Default|SetDissplacementX 22.0)
          (Variables|Default|SetDissplacementZ -38.0))
        (:3
          (Variables|Default|SetDissplacementX -22.0)
          (Variables|Default|SetDissplacementZ -38.0))
        (:4
          (Variables|Default|SetDissplacementX -44.0)
          (Variables|Default|SetDissplacementZ 0.0))
        (:5
          (Variables|Default|SetDissplacementX -22.0)
          (Variables|Default|SetDissplacementZ 38.0)))
      (Default|MovetoBot (Utilities|Array|Get(acopy) _bossshieldbubble _output_get) (+ (Variables|Default|GetDissplacementX) (Variables|Default|GetMinion2X)) (+ (Variables|Default|GetDissplacementZ) (Variables|Default|GetMinion2Z)) (stale Custom|SpawnBot _returnvalue))
      (Utilities|Array|RemoveIndex _bossshieldbubble _output_get))
    (Utilities|Array|AddUnique (Variables|Default|GetMinions_2) (stale Custom|SpawnBot _returnvalue))))

(event Custom|ChooseSunPosition
  ;[1 1 1] ChooseSunPosition
  (switch int (Math|Random|RandomIntegerinRange 0 8)
    (:0
      (CallFunction|SpawnSunMarkerandSEndONposition 0.0 3e+02))
    (:1
      (CallFunction|SpawnSunMarkerandSEndONposition 3e+02 0.0))
    (:2
      (CallFunction|SpawnSunMarkerandSEndONposition -3e+02 0.0))
    (:3
      (CallFunction|SpawnSunMarkerandSEndONposition 3e+02 3e+02))
    (:4
      (CallFunction|SpawnSunMarkerandSEndONposition -3e+02 0.0))
    (:5
      (CallFunction|SpawnSunMarkerandSEndONposition 0.0 1.5e+02))))

(event EventBeginPlay
  ;[1 1 1] BeginPlay
)

(event EventTick
  (params (DeltaSeconds :type Float%20%28single-precision%29))
  ;[1 1 1] EventTick
  (Utilities|FlowControl|Sequence
    (:then_0
      (if (<= (Variables|Default|GetHealth) 0.0)
        (CallFunction|BossDeath)))
    (:then_1
      (if (>= (Variables|Default|GetMinion2RespawnCooldown) 1.0)
        (if (Variables|Default|GetSpawn1Minion)
          (Variables|Default|SetMinion2RespawnCooldown 0.0)
          (CallFunction|1AttackBotSequence)
          (Variables|Default|SetSpawn1Minion false)
          (else
            (Variables|Default|SetMinion2RespawnCooldown 0.0)
            (CallFunction|2AttackBotSequence)
            (Variables|Default|SetSpawn1Minion true)))))
    (:then_2
      (if (and (Variables|Default|GetBossNotRecharging) (== (Utilities|Array|Length (Variables|Default|GetBossShieldBubble)) 0))
        (CallFunction|StartChargingShield)))
    (:then_3
      (if (and (Variables|Default|GetBombersNotSpawnedYet) (<= (Variables|Default|GetHealth) 0.67))
        (Default|CallBombers (Variables|Default|GetRefToBossManager))
        (Variables|Default|SetBombersNotSpawnedYet false)))
    (:then_4
      (if (and (<= (Variables|Default|GetHealth) 0.34) (Variables|Default|GetIsSunPhaseDisabled))
        (CallFunction|SunGeneratingPhase)
        (Variables|Default|SetIsSunPhaseDisabled false)))
    (:then_5
      (if (>= (Variables|Default|GetSunREspawnCooldown) 1.0)
        (Variables|Default|SetSunREspawnCooldown 0.0)
        (CallFunction|ChooseSunPosition)))))

(fn ConstructionScript
  (bind _outactors (Actor|GetAllActorsOfClass "/Game/MYContent/Blueprints/BP_Canon.BP_Canon_C"))
  (Variables|Default|SetRefToCannon (Utilities|Array|Get(acopy) _outactors))
  (bind _outactors_2 (Actor|GetAllActorsOfClass "/Game/MYContent/Blueprints/BossFightManager.BossFightManager_C"))
  (Variables|Default|SetRefToBossManager (Utilities|Array|Get(acopy) _outactors_2)))