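; BP_RocketManager is a manager actor that spawns replacement rockets aimed at the cannon.
; On BeginPlay it caches the first BP_Canon found in the level.
; RespawnRocket spawns a BP_NewRocket at the given location, always ignoring collisions, rotated by look-at toward the cannon's Cube component.
; A 270-degree pitch offset is added to that look-at rotation.
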(event Custom|RespawnRocket
  (params (WhereRespawn :type Vector))
  (bind _cannon (Variables|Default|GetCannon))
  (bind _cube (Variables|/Game/MYContent/Blueprints/BP_Canon.BP_Canon_C|GetCube _cannon))
  (bind _returnvalue (Transformation|GetWorldTransform _cube))
  (bind _returnvalue_2 (Math|Rotator|FindLookatRotation (Math|Vector|MakeVector (.x WhereRespawn) (.y WhereRespawn) (.z WhereRespawn)) (Math|Vector|MakeVector (.x (.location _returnvalue)) (.y (.location _returnvalue)) (.z (.location _returnvalue)))))
  (bind (_roll _pitch _yaw) (Math|Rotator|BreakRotator _returnvalue_2))
  ;[1 1 1] RespawnRocketAtLocation
  (Game|SpawnActorfromClass "/Game/MYContent/Blueprints/ART/BP_NewRocket.BP_NewRocket_C" (Math|Transform|MakeTransform (Math|Vector|MakeVector (.x WhereRespawn) (.y WhereRespawn) (.z WhereRespawn)) (Math|Rotator|MakeRotator _roll (+ _pitch 2.7e+02) _yaw) "1,1,1") "AlwaysSpawn" 0 0))

(event EventBeginPlay
  ;[1 1 1] BeginPlay
  (bind _outactors (Actor|GetAllActorsOfClass "/Game/MYContent/Blueprints/BP_Canon.BP_Canon_C"))
  (Variables|Default|SetCannon (Utilities|Array|Get(acopy) _outactors)))

(fn ConstructionScript)