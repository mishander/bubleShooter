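; Boss fight manager that stages the encounter's opening when play begins.
; Its construction script caches the boss, cannon and playfield's interface through GetAllActorsOfClass.
; BeginPlay starts a timeline that lowers the boss by a fixed step per update until it reaches a height threshold, plays a world camera shake and shows player and boss health.
; It then spawns a minion, tracks it in an array and orients it toward the cannon with a pitch offset.
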(event Custom|SetUpBossPosition
  (bind _reftoboss (Variables|Default|GetrefToBoss))
  ;[1 1 1] SetUPBossPosition
  (Timeline|Timeline_0 PlayFromStart
    (:Update
      (Transformation|AddActorWorldOffset _reftoboss "0, 0,-0.750000")
      (if (<= (.z (Transformation|GetActorLocation _reftoboss)) 8.4e+02)
        (Timeline|Timeline_0 Stop)))))

(event Custom|Set%20up%20Minion%20Position
  (params (LinearPosition :type Vector) (RefToMinion :type BP%20Minion%20Object%20Reference))
  (bind _reftocannon (Variables|Default|GetRefToCannon))
  (bind _returnvalue (Transformation|GetActorLocation _reftocannon))
  (bind _returnvalue_2 (Math|Rotator|FindLookatRotation (Math|Vector|MakeVector (.x LinearPosition) (.y LinearPosition) (.z LinearPosition)) _returnvalue))
  (bind (_roll _pitch _yaw) (Math|Rotator|BreakRotator _returnvalue_2))
  ;[1 1 1] Set up Minions Position
  (Transformation|SetActorLocation RefToMinion (Math|Vector|MakeVector (.x LinearPosition) (.y LinearPosition) (.z LinearPosition)) false false)
  (Transformation|SetActorRotation RefToMinion (Math|Rotator|MakeRotator _roll (+ _pitch 2.7e+02) _yaw)))

(event Custom|BossShake
  ;[1 1 1] Boss Shake
  (Camera|PlayWorldCameraShake "/Game/MYContent/Blueprints/Shakes/BossRespawnameraShake.BossRespawnameraShake_C" "0.000000,387.000000,190.000000" 5e+02 5e+02))

(event Custom|Respawn%20Minions
  (params (Number :type Integer))
  ;[1 1 1] RespawnMinions
  (for _index (range 1 Number)
    (bind _returnvalue (Game|SpawnActorfromClass "/Game/MYContent/Blueprints/BP_Minion.BP_Minion_C" (Math|Transform|MakeTransform "200.000000,0.000000,200.000000" "0.000000, 0, 0" "1,1,1") "AlwaysSpawn" 0 0))
    (Utilities|Array|AddUnique (Variables|Default|GetArrayOfMinions) _returnvalue)))

(event EventBeginPlay
  ;[1 1 1] BeginPlay
  (CallFunction|SetUpBossPosition)
  (CallFunction|BossShake)
  (Utilities|FlowControl|Delay 0.0)
  (Default|ShoworHidePlayerAnBossHealth (Variables|Default|GetRefToInterface) true)
  (CallFunction|RespawnMinions 1)
  (CallFunction|SetUpMinionPosition "200.000000, 0,200.000000" (Utilities|Array|Get(acopy) (Variables|Default|GetArrayOfMinions))))

(fn ConstructionScript
  (bind _outactors (Actor|GetAllActorsOfClass "/Game/MYContent/Blueprints/BP_BOSS.BP_BOSS_C"))
  (Variables|Default|SetrefToBoss (Utilities|Array|Get(acopy) _outactors))
  (bind _outactors_2 (Actor|GetAllActorsOfClass "/Game/MYContent/Blueprints/BP_PlayFieldConstructror.BP_PlayFieldConstructror_C"))
  (Variables|Default|SetRefToInterface (Variables|/Game/MYContent/Blueprints/BP_PlayFieldConstructror.BP_PlayFieldConstructror_C|GetRefToInterface (Utilities|Array|Get(acopy) _outactors_2)))
  (bind _outactors_3 (Actor|GetAllActorsOfClass "/Game/MYContent/Blueprints/BP_Canon.BP_Canon_C"))
  (Variables|Default|SetRefToCannon (Utilities|Array|Get(acopy) _outactors_3)))